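; Gameplay ability that equips the hero's axe.
; It plays the equip montage, waits for the Player.Event.Equip.Axe event, then snaps the carried axe to the right-hand socket and sets it as the equipped weapon tag.
; HandleEquipWeapon links the weapon's anim layer, adds its input mapping context and grants its abilities, storing the spec handles on the weapon.
; The ability ends when the montage completes, blends out or is interrupted or cancelled.
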(event `self.K2_ActivateAbility`
  ; Play the animation montage, and wait till we recieve a event gameplay tag
  (`AbilityTask_PlayMontageAndWait.CreatePlayMontageAndWaitProxy` "None" "/Game/PlayerCharacter/Montages/AM_Hero_Axe_Equip.AM_Hero_Axe_Equip"
    (:`then`
      (`AbilityTask_WaitGameplayEvent.WaitGameplayEvent` (struct :`TagName` "Player.Event.Equip.Axe") null
        (:`EventReceived`
          ; Attach weapon to Actor
          (`Actor.K2_AttachToComponent` (`PawnCombatComponent.GetCharacterCarriedWeaponByTag` (`self.GetHeroCombatComponentFromActorInfo`) (struct :`TagName` "Player.Weapon.Axe")) (`self.GetOwningComponentFromActorInfo`) "AxeRightHandSocket" "SnapToTarget" "KeepRelative" "KeepWorld" true)
          (`self.HandleEquipWeapon` (`HeroCombatComponent.GetHeroCarriedWeaponByTag` (`self.GetHeroCombatComponentFromActorInfo`) (struct :`TagName` "Player.Weapon.Axe")))
          (set `PawnCombatComponent.CurrentEquippedWeaponTag` (struct :`TagName` "Player.Weapon.Axe") (`self.GetHeroCombatComponentFromActorInfo`)))))
    (:`OnCompleted`
      (`self.K2_EndAbility` :!label _label))
    (:`OnBlendOut`
      (goto _label))
    (:`OnInterrupted`
      (goto _label))
    (:`OnCancelled`
      (goto _label))))

(fn `HandleEquipWeapon`
  (params (WeaponToEquip :type "ActionGameHeroWeapon Object Reference"))
  (locals (CachedHeroWeaponData :type "ActionGameHeroWeaponData Structure"))
  (set `local.CachedHeroWeaponData` (`ActionGameHeroWeapon.HeroWeaponData` WeaponToEquip))
  (`|ExecutionSequence`
    (:`then_0`
      ; Link Animation layer of the specific weapon
      (`SkeletalMeshComponent.LinkAnimClassLayers` (`self.GetOwningComponentFromActorInfo`) (`.WeaponAnimLayerToLink` (break `ActionGameHeroWeaponData` (`local.CachedHeroWeaponData`)))))
    (:`then_1`
      (`EnhancedInputSubsystemInterface.AddMappingContext` (pcsubsystem `EnhancedInputLocalPlayerSubsystem` (`self.GetHeroControllerFromActorInfo`)) (`.WeaponInputMappingContext` (break `ActionGameHeroWeaponData` (`local.CachedHeroWeaponData`))) 1 (struct)))
    (:`then_2`
      (bind _outgrantedabilityspechandle (`ActionGameAbilitySystemComponent.GrantHeroWeaponAbilities` (`self.GetActionGameAbilitySystemComponentFromActorInfo`) (`.DefaultWeaponAbilities` (break `ActionGameHeroWeaponData` (`local.CachedHeroWeaponData`))) (`self.GetAbilityLevel`)))
      (`ActionGameHeroWeapon.AssignGrantedAbilitySpecHandle` (`local.WeaponToEquip`) _outgrantedabilityspechandle))))